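; BP_PerkLibFunctionLibrary is the function library of PerkLib, a mod library by Deltin for creating and looking up perks.
; CreateFloatPerk finds the InitSpacerig actor in the level and forwards the float perk to its AddFloatPerk.
; GetPerkBySavegameID linearly searches the FSD game data perk assets for a matching savegame ID and returns whether it exists, with the asset.
; PerkLibModInfo reports the mod's name, author and version.
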(fn CreateFloatPerk
  (params (Float%20Perk :type F%20Modded%20Float%20Perk%20Structure))
  (bind _returnvalue (Actor|GetActorOfClass 0 "/Game/PerkLib/InitSpacerig.InitSpacerig_C"))
  (Default|AddFloatPerk _returnvalue Float%20Perk))

(fn GetPerkbySavegameID
  (params (Savegame%20ID :type Guid%20Structure))
  (for _array_element (Utilities|Struct|BreakGDPerks (Variables|/Script/FSD.GameData|Getperks (Class|GameFunctionLibrary|GetFSDGameData)))
    (if (== (Variables|/Script/FSD.PerkAsset|GetSavegameID _array_element) Savegame%20ID)
      (return true _array_element)))
  (return false 0))

(fn PerkLibModInfo
  (return "PerkLib" "Deltin" "v1.0"))